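; Katana player character Blueprint with target lock, directional evade and an equip toggle, still carrying debug prints.
; R sphere-traces along camera forward to set or clear HitActor, which Tick turns character and controller toward.
; A LockOn branch trails the spring arm and frames the target from behind, but nothing connected sets LockOn true.
; Space plays an evade montage section chosen by WalkingDirectionAngle; construction tints mesh materials yellow.
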(event EventBeginPlay)

(event Collision|EventActorBeginOverlap
  (params (OtherActor :type Actor%20Object%20Reference)))

(event EventTick
  (params (DeltaSeconds :type Float%20%28single-precision%29))
  (bind _returnvalue (Transformation|GetActorLocation))
  (bind _returnvalue_2 (Transformation|GetActorLocation))
  (bind _camera (Variables|Default|GetCamera))
  (bind _springarm (Variables|Default|GetSpringArm))
  (Utilities|FlowControl|Sequence
    (:then_0
      (bind _hit_actor (Variables|Default|GetHit%20Actor)
        (:then
          (Transformation|SetActorRotation self (Math|Rotator|FindLookatRotation (Math|Vector|MakeVector (.x _returnvalue_2) (.y _returnvalue_2) 0.0) (Math|Vector|MakeVector (.x (Transformation|GetActorLocation _hit_actor)) (.y (Transformation|GetActorLocation _hit_actor)) 0.0)))
          (Transformation|SetActorRotation (Pawn|GetController) (Math|Rotator|FindLookatRotation (Math|Vector|MakeVector (.x _returnvalue_2) (.y _returnvalue_2) 0.0) (Math|Vector|MakeVector (.x (Transformation|GetActorLocation _hit_actor)) (.y (Transformation|GetActorLocation _hit_actor)) 0.0))))
        (:else)))
    (:then_1
      (if (Variables|Default|GetbLockOn)
        (Transformation|SetWorldLocation _springarm (Math|Vector|Lerp(Vector) (Transformation|GetWorldLocation (Variables|Default|GetSpringArm)) (Transformation|GetActorLocation) 0.03) false false)
        (bind _hit_actor_2 (Variables|Default|GetHit%20Actor)
          (:then
            (Transformation|SetWorldLocation _camera (+ (+ (Transformation|GetWorldLocation _springarm) (* (Math|Vector|GetForwardVector (Math|Rotator|FindLookatRotation (Math|Vector|MakeVector (.x _returnvalue) (.y _returnvalue) 0.0) (Math|Vector|MakeVector (.x (Transformation|GetActorLocation _hit_actor_2)) (.y (Transformation|GetActorLocation _hit_actor_2)) 0.0))) -1.0 3e+02)) "0.000000,0.000000,90.000000") false false)
            (Transformation|SetWorldRotation _camera (Math|Rotator|FindLookatRotation (Math|Vector|MakeVector (.x _returnvalue) (.y _returnvalue) 0.0) (Math|Vector|MakeVector (.x (Transformation|GetActorLocation _hit_actor_2)) (.y (Transformation|GetActorLocation _hit_actor_2)) 0.0)) false false))
          (:else))
        (else
          (Transformation|SetWorldLocation (Variables|Default|GetSpringArm) (Transformation|GetActorLocation) false false))))
    (:then_2
      (Development|PrintString (Utilities|String|ToString(Float) (Variables|Default|GetWalkingDirectionAngle))))))

(event Input|KeyboardEvents|DebugKeySpaceBar
  (params (Key :type Key%20Structure :default "None") (ActionValue :type Input%20Action%20Value%20Structure))
  (:Pressed
    (bind _slotname (CallFunction|SelectSlot))
    (Animation|PlayAnimMontage "/Game/_dev/Actor/Character/Player/Katana/Animation/Movement/Katana_Evade.Katana_Evade" 1.0 _slotname)))

(event Input|KeyboardEvents|X
  (params (Key :type Key%20Structure :default "None"))
  (:Pressed
    (bind _isa (Utilities|FlowControl|FlipFlop)
      (:A
        _)
      (:B
        _))
    (Variables|Default|SetbEquipState _isa)
    (Development|PrintString "Hello")))

(event Input|KeyboardEvents|R
  (params (Key :type Key%20Structure :default "None"))
  (bind _returnvalue (Transformation|GetActorLocation))
  (bind _camera (Variables|Default|GetCamera))
  (bind _returnvalue_2 (Math|Vector|GetForwardVector _camera))
  (:Pressed
    (Development|PrintString "World")
    (bind (_outhit _returnvalue_3) (Collision|SphereTraceForObjects _returnvalue (+ _returnvalue (* (Math|Vector|MakeVector (.x _returnvalue_2) (.y _returnvalue_2) 0.0) 1e+03)) 5e+01 (Utilities|Array|MakeArray "ObjectTypeQuery3") false 0 "ForDuration"))
    (if _returnvalue_3
      (Development|PrintString "Hello")
      (Variables|Default|GetHit%20Actor
        (:then
          (Variables|Default|SetHit%20Actor 0)
          (Variables|Default|SetbLockOn false :!label _label))
        (:else
          (Variables|Default|SetHit%20Actor (.HitActor (Collision|BreakHitResult _outhit)))))
      (else
        (Variables|Default|SetHit%20Actor 0)
        (goto _label)))))

(fn ConstructionScript
  (for (_array_element _array_index) (Rendering|Material|GetMaterials (Variables|Character|GetMesh))
    (bind _returnvalue (Rendering|Material|CreateDynamicMaterialInstance (Variables|Character|GetMesh) _array_index _array_element "None" :!class /Script/Engine.PrimitiveComponent))
    (Rendering|Material|SetVectorParameterValue _returnvalue "Color" "(R=1.000000,G=1.000000,B=0.000000,A=1.000000)" :!class /Script/Engine.MaterialInstanceDynamic)))

(fn SelectSlot
  (Utilities|FlowControl|Sequence
    (:then_0
      (if (Math|Float|InRange(Float) (Variables|Default|GetWalkingDirectionAngle) -45.0 45.0)
        (LocalVariables|SetLocalIndex 0)
        (return (Utilities|Select :Index (LocalVariables|GetLocalIndex) :Option%200 "FWD" :Option%201 "Right" :Option%202 "BWD" :Option%203 "Left"))
        (elif (Math|Float|InRange(Float) (Variables|Default|GetWalkingDirectionAngle) 45.0 135.0 false)
          (LocalVariables|SetLocalIndex 1)
          (return (Utilities|Select :Index (LocalVariables|GetLocalIndex) :Option%200 "FWD" :Option%201 "Right" :Option%202 "BWD" :Option%203 "Left"))
          (elif (or (Math|Float|InRange(Float) (Variables|Default|GetWalkingDirectionAngle) 135.0 1.8e+02 false) (Math|Float|InRange(Float) (Variables|Default|GetWalkingDirectionAngle) -1.8e+02 -135.0 true false))
            (LocalVariables|SetLocalIndex 2)
            (return (Utilities|Select :Index (LocalVariables|GetLocalIndex) :Option%200 "FWD" :Option%201 "Right" :Option%202 "BWD" :Option%203 "Left"))
            (elif (Math|Float|InRange(Float) (Variables|Default|GetWalkingDirectionAngle) -135.0 -45.0 false)
              (LocalVariables|SetLocalIndex 3)
              (return (Utilities|Select :Index (LocalVariables|GetLocalIndex) :Option%200 "FWD" :Option%201 "Right" :Option%202 "BWD" :Option%203 "Left")))))))))