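; Player Assassin character Blueprint that maps input to evade, attack, block, equip toggle and lock-on, and creates the in-game status UI on BeginPlay.
; Space picks a directional evade montage from the walking angle and starts a timeline, while right mouse drives upper-body weight for blocking.
; R calls LockOn; the local target-trace and lock-on camera logic is disconnected, and Tick is empty.
; The construction script tints all mesh materials blue through dynamic instances.
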(event `Key|SpaceBar`
  (params (Key :type "Key Structure"))
  (:`Pressed`
    (switch `int` (`KismetMathLibrary.FTrunc` (/ (`self.WalkingDirectionAngle`) 72.0))
      (:`-2`
        (set `self.Evade` "/Game/Retargeted_Asset/Retarget_Assassin/Frank_RPG_Assassin_Evade_B_IP_Montage.Frank_RPG_Assassin_Evade_B_IP_Montage"))
      (:`-1`
        (set `self.Evade` "/Game/Retargeted_Asset/Retarget_Assassin/Frank_RPG_Assassin_Evade_L_IP_Montage.Frank_RPG_Assassin_Evade_L_IP_Montage"))
      (:`0`
        (set `self.Evade` "/Game/Retargeted_Asset/Retarget_Assassin/Frank_RPG_Assassin_Evade_F_IP_Montage.Frank_RPG_Assassin_Evade_F_IP_Montage"))
      (:`1`
        (set `self.Evade` "/Game/Retargeted_Asset/Retarget_Assassin/Frank_RPG_Assassin_Evade_R_IP_Montage.Frank_RPG_Assassin_Evade_R_IP_Montage")))
    (`|PlayMontage` (`self.Mesh`) (`self.Evade`)
      (:`then`
        (`Timeline|타임라인` :!via `PlayFromStart`)))))

(event `self.ReceiveBeginPlay`
  (set `self.bLockOn` false)
  (set `self.CharacterRotationAlphaLinearValue` 5.0)
  (bind _asbase_player_controller (cast `BasePlayerController` (`GameplayStatics.GetPlayerController` 0)))
  (set `self.As Base Player Controller` _asbase_player_controller)
  (bind _returnvalue (`|CreateWidget` "/Game/_dev/UI/UI_InGame.UI_InGame_C"))
  (bind _output_get (set `self.StatusUI` _returnvalue))
  (`UserWidget.AddToViewport` _returnvalue 0)
  (`UserWidget.AddToViewport` _output_get 0))

(event `self.ReceiveTick`
  (params (DeltaSeconds :type "Float (single-precision)")))

(event `Key|RightMouseButton`
  (params (Key :type "Key Structure"))
  (:`Pressed`
    (set `self.UpperWeight` 1.0)
    (`|PlayMontage` null "/Game/Retargeted_Asset/Retarget_Assassin/Frank_RPG_Assassin_Block_Montage.Frank_RPG_Assassin_Block_Montage"))
  (:`Released`
    (set `self.UpperWeight` 0.0)))

(event `Key|X`
  (params (Key :type "Key Structure"))
  (:`Pressed`
    (bind _isa (`/Engine/EditorBlueprintResources/StandardMacros.FlipFlop`)
      (:`A`
        _)
      (:`B`
        _))
    (set `self.bEquipState` _isa)))

(event `Key|R`
  (params (Key :type "Key Structure"))
  (:`Pressed`
    (`self.LockOn`)))

(event `Key|E`
  (params (Key :type "Key Structure"))
  (:`Pressed`
    (`|PlayMontage` (`self.Mesh`) "/Game/Retargeted_Asset/Retarget_Assassin/Frank_RPG_Assassin_Attack02_IP1_Montage.Frank_RPG_Assassin_Attack02_IP1_Montage")))

(fn `UserConstructionScript`
  (for (_array_element _array_index) (`MeshComponent.GetMaterials` (`self.Mesh`))
    (bind _returnvalue (`PrimitiveComponent.CreateDynamicMaterialInstance` (`self.Mesh`) _array_index _array_element "None"))
    (`MaterialInstanceDynamic.SetVectorParameterValue` _returnvalue "Color" (struct :`B` 1.0 :`A` 1.0))))