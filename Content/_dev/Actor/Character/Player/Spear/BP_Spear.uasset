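; BP_Spear is a spear-wielding player actor that plays skill montages from the Q key.
; Pressing Q while Throwing is set plays the jump montage and clears both throw flags, then a montage notify sets Throwable.
; Releasing Q while Throwing is clear plays the Skill01 montage, clearing both flags on completion.
; The construction script gives each mesh material a dynamic instance tinted green.
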(event `self.ReceiveBeginPlay`)

(event `Key|Q`
  (params (Key :type "Key Structure"))
  (:`Pressed`
    (if (`self.bThrowing`)
      (`|PlayMontage` (`self.Mesh`) "/Game/Retargeted_Asset/Retarget_Spear/Spear_SkillJump_Montage.Spear_SkillJump_Montage"
        (:`then`
          (set `self.bThrowable` false)
          (set `self.bThrowing` false))
        (:`OnNotifyBegin`
          (set `self.bThrowable` true)))))
  (:`Released`
    (if (not (`self.bThrowing`))
      (`|PlayMontage` (`self.Mesh`) "/Game/Retargeted_Asset/Retarget_Spear/Spear_Skill01_Montage.Spear_Skill01_Montage"
        (:`OnCompleted`
          (set `self.bThrowing` false)
          (set `self.bThrowable` false))))))

(fn `UserConstructionScript`
  (for (_array_element _array_index) (`MeshComponent.GetMaterials` (`self.Mesh`))
    (bind _returnvalue (`PrimitiveComponent.CreateDynamicMaterialInstance` (`self.Mesh`) _array_index _array_element "None"))
    (`MaterialInstanceDynamic.SetVectorParameterValue` _returnvalue "Color" (struct :`G` 1.0 :`A` 1.0))))